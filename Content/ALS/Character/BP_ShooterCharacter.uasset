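; Player shooter character handling Enhanced Input movement, look, aiming and switching between unarmed, pistol and rifle.
; Weapon switching sets the equipped gun and links a matching animation class layer to the mesh.
; Aiming toggles the gate (gait) through UpdateGate, which notifies the AnimInstance and applies that gate's speed, acceleration and braking from a settings map to CharacterMovement.
; Debug keys toggle global slow motion.
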(event Input|EnhancedActionEvents|EnhancedInputActionIA_SwitchWeapon
  (params (ActionValue :type Float%20%28double-precision%29) (ElapsedSeconds :type Float%20%28double-precision%29) (TriggeredSeconds :type Float%20%28double-precision%29) (InputAction :type Input%20Action%20Object%20Reference :default "/Game/ALS/Inputs/InputActions/IA_SwitchWeapon.IA_SwitchWeapon"))
  (bind _mesh (Variables|Character|GetMesh))
  ;[0 0.6192 1] Switch Weapon Event
  (:Triggered
    (Utilities|FlowControl|DoOnce false :!label _label
      (:Completed
        (switch int (Math|Float|Truncate ActionValue)
          (:1
            (Variables|Gun|SetEquippedGun "NewEnumerator0")
            (Components|SkeletalMesh|AnimationBlueprintLinking|LinkAnimClassLayers _mesh "/Game/ALS/AnimationBlueprints/ABP_UnArmed.ABP_UnArmed_C"))
          (:2
            (Variables|Gun|SetEquippedGun "NewEnumerator1")
            (Components|SkeletalMesh|AnimationBlueprintLinking|LinkAnimClassLayers _mesh "/Game/ALS/AnimationBlueprints/ABP_Pistol.ABP_Pistol_C"))
          (:3
            (Variables|Gun|SetEquippedGun "NewEnumerator2")
            (Components|SkeletalMesh|AnimationBlueprintLinking|LinkAnimClassLayers _mesh "/Game/ALS/AnimationBlueprints/ABP_Rifle.ABP_Rifle_C"))))))
  (:Completed
    (goto _label Reset)))

(event Input|EnhancedActionEvents|EnhancedInputActionIA_Look
  (params (ActionValue :type Vector%202D%20Structure) (ElapsedSeconds :type Float%20%28double-precision%29) (TriggeredSeconds :type Float%20%28double-precision%29) (InputAction :type Input%20Action%20Object%20Reference :default "/Game/ALS/Inputs/InputActions/IA_Look.IA_Look"))
  (bind (_x _y) (Math|Vector2D|BreakVector2D ActionValue))
  ;[0 0.6172 1] Look Functionality
  (Pawn|Input|AddControllerYawInput _x)
  (Pawn|Input|AddControllerPitchInput _y))

(event Input|EnhancedActionEvents|EnhancedInputActionIA_Move
  (params (ActionValue :type Vector%202D%20Structure) (ElapsedSeconds :type Float%20%28double-precision%29) (TriggeredSeconds :type Float%20%28double-precision%29) (InputAction :type Input%20Action%20Object%20Reference :default "/Game/ALS/Inputs/InputActions/IA_Move.IA_Move"))
  (bind (_x _y) (Math|Vector2D|BreakVector2D ActionValue))
  (bind _returnvalue (Pawn|GetControlRotation :!class /Script/Engine.Pawn))
  ;[0 0.6172 1] Move Functionality
  (Utilities|FlowControl|Sequence
    (:then_0
      (Pawn|Input|AddMovementInput (Math|Vector|GetRightVector (Math|Rotator|MakeRotator (.roll _returnvalue) 0.0 (.yaw _returnvalue))) _x false))
    (:then_1
      (Pawn|Input|AddMovementInput (Math|Vector|GetForwardVector (Math|Rotator|MakeRotator 0.0 0.0 (.yaw (Pawn|GetControlRotation :!class /Script/Engine.Pawn)))) _y false))))

(event Input|EnhancedActionEvents|EnhancedInputActionIA_Aim
  (params (ActionValue :type Boolean) (ElapsedSeconds :type Float%20%28double-precision%29) (TriggeredSeconds :type Float%20%28double-precision%29) (InputAction :type Input%20Action%20Object%20Reference :default "/Game/ALS/Inputs/InputActions/IA_Aim.IA_Aim"))
  ;[0 0.6172 1] Aim Functionality
  (:Started
    (Gate|UpdateGate "NewEnumerator0"))
  (:Completed
    (Gate|UpdateGate "NewEnumerator1")))

(event EventBeginPlay
  ;[0.004834 1 0.5158] Begin Play Init
  (bind _asplayer_controller (Utilities|Casting|CastToPlayerController (Pawn|GetController)))
  (Input|AddMappingContext (PlayerController|LocalPlayerSubsystems|GetEnhancedInputLocalPlayerSubsystem _asplayer_controller) "/Game/ALS/Inputs/IMC_ALS.IMC_ALS" 0 "(bIgnoreAllPressedKeysUntilRelease=True,bForceImmediately=False,bNotifyUserSettings=False)")
  (Components|SkeletalMesh|AnimationBlueprintLinking|LinkAnimClassLayers (Variables|Character|GetMesh) "/Game/ALS/AnimationBlueprints/ABP_UnArmed.ABP_UnArmed_C")
  (Gate|UpdateGate "NewEnumerator1"))

(event Input|KeyboardEvents|DebugKeySubtract
  (params (Key :type Key%20Structure :default "None") (ActionValue :type Input%20Action%20Value%20Structure))
  ;[0.9043 0.06815 0.1564 0.5] Time Dilation Debug Settings
  (:Pressed
    (Utilities|Time|SetGlobalTimeDilation 0.1)))

(event Input|KeyboardEvents|DebugKeyAdd
  (params (Key :type Key%20Structure :default "None") (ActionValue :type Input%20Action%20Value%20Structure))
  ;[0.9043 0.06815 0.1564 0.5] Time Dilation Debug Settings
  (:Pressed
    (Utilities|Time|SetGlobalTimeDilation 1.0)))

(fn ConstructionScript)

(fn UpdateGate
  (params (Gate :type E_Gate%20Enum :default "NewEnumerator0"))
  (Variables|Gate|SetCurrentGate Gate)
  (Class|BPIAnimationBlueprintInterface|RecieveCurrentGate(Message) (Components|SkeletalMesh|GetAnimInstance (Variables|Character|GetMesh)) Gate)
  (Utilities|FlowControl|Sequence
    (:then_0
      (Variables|/Script/Engine.CharacterMovementComponent|SetMaxWalkSpeed (Variables|Character|GetCharacterMovement) (.MaxWalkSpeed (Utilities|Struct|BreakS_GateSetting (.Value (Utilities|Map|Find (Variables|Gate|GetGateSettings) (Variables|Gate|GetCurrentGate)))))))
    (:then_1
      (Variables|/Script/Engine.CharacterMovementComponent|SetMaxAcceleration (Variables|Character|GetCharacterMovement) (.MaxAcceleration (Utilities|Struct|BreakS_GateSetting (.Value (Utilities|Map|Find (Variables|Gate|GetGateSettings) (Variables|Gate|GetCurrentGate)))))))
    (:then_2
      (Variables|/Script/Engine.CharacterMovementComponent|SetBrakingDecelerationWalking (Variables|Character|GetCharacterMovement) (.MaxDecelerationWalking (Utilities|Struct|BreakS_GateSetting (.Value (Utilities|Map|Find (Variables|Gate|GetGateSettings) (Variables|Gate|GetCurrentGate)))))))
    (:then_3
      (Variables|/Script/Engine.CharacterMovementComponent|SetBrakingFrictionFactor (Variables|Character|GetCharacterMovement) (.BrakingFrictionFactor (Utilities|Struct|BreakS_GateSetting (.Value (Utilities|Map|Find (Variables|Gate|GetGateSettings) (Variables|Gate|GetCurrentGate)))))))
    (:then_4
      (Variables|/Script/Engine.CharacterMovementComponent|SetBrakingFriction (Variables|Character|GetCharacterMovement) (.BrakingFriction (Utilities|Struct|BreakS_GateSetting (.Value (Utilities|Map|Find (Variables|Gate|GetGateSettings) (Variables|Gate|GetCurrentGate)))))))
    (:then_5
      (Variables|/Script/Engine.CharacterMovementComponent|SetbUseSeparateBrakingFriction (Variables|Character|GetCharacterMovement) (.UseSeperateBrakingFriction (Utilities|Struct|BreakS_GateSetting (.Value (Utilities|Map|Find (Variables|Gate|GetGateSettings) (Variables|Gate|GetCurrentGate)))))))))